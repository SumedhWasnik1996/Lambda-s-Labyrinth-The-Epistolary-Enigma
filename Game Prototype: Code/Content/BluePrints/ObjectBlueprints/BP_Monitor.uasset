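; BP_Monitor is an interactable monitor that opens the Lexicon puzzle interface.
; Show and hide prompt events toggle its prompt widget's visibility with debug prints.
; Interact creates UMG_LexiconInterface, passes it a reference to the monitor, switches input to UI only with a cursor, and hides the prompt.
; FinalReductionCompete is the puzzle-solved hook, which currently only prints a message.
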(event EventBeginPlay)

(event Collision|EventActorBeginOverlap
  (params (OtherActor :type Actor%20Object%20Reference)))

(event EventTick
  (params (DeltaSeconds :type Float%20%28single-precision%29)))

(event EventShowInteractionPrompt
  (params (InteractActor :type Actor%20Object%20Reference))
  (Development|PrintString "EVENT FIRED : Showing Interaction Prompt" true true "(R=0.079554,G=1.000000,B=0.006672,A=1.000000)")
  (Rendering|SetVisibility (Variables|Default|GetPromptWidget) true false))

(event EventHideInteractionPrompt
  (Development|PrintString "EVENT FIRED : Hiding Interaction Prompt" true true "(R=1.000000,G=0.006903,B=0.000000,A=1.000000)")
  (Rendering|SetVisibility (Variables|Default|GetPromptWidget) false false))

(event EventInteract
  (params (InteractingActor :type Actor%20Object%20Reference))
  (bind _returnvalue (Game|GetPlayerController 0))
  (bind _returnvalue_2 (UserInterface|CreateWidget "/Game/UI/UMG_LexiconInterface.UMG_LexiconInterface_C"))
  (bind _output_get (Variables|Default|SetLexiconUI _returnvalue_2))
  (Default|SetMonitorReference _output_get self)
  (UserInterface|Viewport|AddtoViewport (Variables|Default|GetLexiconUI) 0)
  (Input|SetInputModeUIOnly _returnvalue (Variables|Default|GetLexiconUI) "DoNotLock" false)
  (Variables|/Script/Engine.PlayerController|SetbShowMouseCursor _returnvalue true)
  (Rendering|SetVisibility (Variables|Default|GetPromptWidget) false false))

(fn ConstructionScript)

(fn FinalReductionCompete
  (Development|PrintString "Puzzle Solved !!!!"))