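; BP_RenamiingPuzzle is a puzzle actor that is solved by entering the correct text answer.
; CheckAnswer compares the input to CorrectAnswer, ignoring case and trailing whitespace, and returns whether they match.
; The first match sets Solved and broadcasts OnPuzzleActorSolved, while later checks only return the comparison result.
; The event graph and construction script hold no logic.
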(event EventBeginPlay)

(event Collision|EventActorBeginOverlap
  (params (OtherActor :type Actor%20Object%20Reference)))

(event EventTick
  (params (DeltaSeconds :type Float%20%28single-precision%29)))

(fn ConstructionScript)

(fn CheckAnswer
  (params (InputAnswer :type Text))
  (bind _returnvalue (Class|KismetTextLibrary|TexttoLower InputAnswer))
  (bind _correctanswer (Variables|Default|GetCorrectAnswer))
  (bind _returnvalue_2 (Class|KismetTextLibrary|TexttoLower _correctanswer))
  (bind _returnvalue_3 (Class|KismetTextLibrary|TextTrimTrailing _returnvalue))
  (bind _returnvalue_4 (Class|KismetTextLibrary|TextTrimTrailing _returnvalue_2))
  (bind _returnvalue_5 (Utilities|Enum|Equal(Enum) _returnvalue_3 _returnvalue_4))
  (if (and (not (Variables|Default|GetbSolved)) _returnvalue_5)
    (Variables|Default|SetbSolved true)
    (Default|CallOnPuzzleActorSolved))
  (return _returnvalue_5))