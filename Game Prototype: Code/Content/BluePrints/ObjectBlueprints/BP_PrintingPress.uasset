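; Interactable printing press actor that presents a number puzzle to the player.
; Interaction prompt events toggle a prompt widget and print debug messages.
; Interact opens UMG_PrintingPressInterface with the correct answer and switches input to UI only.
; OnPuzzleSolved prints a placeholder message and destroys the actor, without restoring the input mode itself.
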(event Custom|OnPuzzleSolved
  (Development|PrintString "A message appears!")
  (Actor|DestroyActor))

(event EventBeginPlay)

(event Collision|EventActorBeginOverlap
  (params (OtherActor :type Actor%20Object%20Reference)))

(event EventTick
  (params (DeltaSeconds :type Float%20%28single-precision%29)))

(event EventShowInteractionPrompt
  (params (InteractActor :type Actor%20Object%20Reference))
  (Development|PrintString "EVENT FIRED : Showing Interaction Prompt" true true "(R=0.079554,G=1.000000,B=0.006672,A=1.000000)")
  (Rendering|SetVisibility (Variables|Default|GetPromptWidget) true false))

(event EventHideInteractionPrompt
  (Development|PrintString "EVENT FIRED : Hiding Interaction Prompt" true true "(R=1.000000,G=0.006903,B=0.000000,A=1.000000)")
  (Rendering|SetVisibility (Variables|Default|GetPromptWidget) false false))

(event EventInteract
  (params (InteractingActor :type Actor%20Object%20Reference))
  (bind _returnvalue (UserInterface|CreateWidget "/Game/UI/UMG_PrintingPressInterface.UMG_PrintingPressInterface_C"))
  (Variables|/Game/UI/UMG_PrintingPressInterface.UMG_PrintingPressInterface_C|SetCorrectNumber _returnvalue (Variables|Default|GetCorrectAnswer))
  (Variables|/Game/UI/UMG_PrintingPressInterface.UMG_PrintingPressInterface_C|SetParentActorRef _returnvalue 0)
  (UserInterface|Viewport|AddtoViewport _returnvalue 0)
  (Input|SetInputModeUIOnly (Game|GetPlayerController 0) _returnvalue "DoNotLock" false))

(fn ConstructionScript)