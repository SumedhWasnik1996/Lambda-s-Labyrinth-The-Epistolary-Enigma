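; BP_PasswordProtectedDrive is an interactable puzzle drive that opens the L3_TrainCarriage level once the player supplies cipher fragments.
; AddFragment stores fragment IDs and calls a completion-check dispatcher, while Interact runs CheckCompletion once fragment counts match.
; CheckCompletion compares both arrays by index, but any single match sets FragCheck and passes; otherwise it clears found fragments.
; Separate events toggle the prompt widget and destroy the drive on final reduction.
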(event Custom|CheckCompletion
  (if (== (Utilities|Array|Length (Variables|Default|GetCipherFragments)) (Utilities|Array|Length (Variables|Default|GetFoundFragments)))
    (for (_array_element _array_index) (Variables|Default|GetCipherFragments)
      (for (_array_element_2 _array_index_2) (Variables|Default|GetFoundFragments)
        (if (== _array_index_2 _array_index)
          (if (Utilities|Enum|Equal(Enum) _array_element_2 _array_element)
            (Variables|Default|SetbFragCheck true)))))
    (if (Variables|Default|GetbFragCheck)
      (Development|PrintString "Frag Check, is Equal")
      (Game|OpenLevel(byObjectReference) "/Game/Maps/L3_TrainCarriage.L3_TrainCarriage")
      (else
        (Development|PrintString "Wrong Fragments " true true "(R=1.000000,G=0.000000,B=0.006408,A=1.000000)")
        (Utilities|Array|Clear (Variables|Default|GetFoundFragments))))))

(event Custom|FinalReductionComplete
  (Development|PrintString "Puzzle Solved! Hard Drive unlocked")
  (Actor|DestroyActor))

(event EventBeginPlay)

(event Collision|EventActorBeginOverlap
  (params (OtherActor :type Actor%20Object%20Reference)))

(event EventTick
  (params (DeltaSeconds :type Float%20%28single-precision%29)))

(event EventShowInteractionPrompt
  (params (InteractActor :type Actor%20Object%20Reference))
  (Rendering|SetVisibility (Variables|Default|GetPromptWidget) true false))

(event EventHideInteractionPrompt
  (Rendering|SetVisibility (Variables|Default|GetPromptWidget) false false))

(event EventInteract
  (params (InteractingActor :type Actor%20Object%20Reference))
  (if (== (Utilities|Array|Length (Variables|Default|GetCipherFragments)) (Utilities|Array|Length (Variables|Default|GetFoundFragments)))
    (CallFunction|CheckCompletion)
    (elif (> (Utilities|Array|Length (Variables|Default|GetCipherFragments)) (Utilities|Array|Length (Variables|Default|GetFoundFragments)))
      (Development|PrintString "Need more Fragments"))))

(fn ConstructionScript)

(fn AddFragment
  (params (FragmentID :type String))
  (Utilities|Array|Add (Variables|Default|GetFoundFragments) FragmentID)
  (Development|PrintString "Fragement Added !!!")
  (Default|CallDispatchCheckCompletion))