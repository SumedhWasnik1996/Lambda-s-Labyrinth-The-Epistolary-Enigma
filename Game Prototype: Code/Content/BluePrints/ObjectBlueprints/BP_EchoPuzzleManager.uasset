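; BP_EchoPuzzleManager is a manager Blueprint that counts solved echo reflection puzzles against a total.
; On BeginPlay it gathers all BP_ReflectionEcho actors, sets the total from their count and calls PuzzleSolved for each, so the solved count immediately reaches the total.
; PuzzleSolved increments the count and checks for completion, but that branch is empty.
; UnifyReflections loops over the reflections with an empty body.
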(event Custom|PuzzleSolved
  (params (ReflectionRef :type BP%20Reflection%20Echo%20Object%20Reference))
  (bind _output_get (Variables|Default|SetSolvedPuzzles (+ (Variables|Default|GetSolvedPuzzles) 1)))
  (if (>= _output_get (Variables|Default|GetTotalPuzzles))
    _))

(event Custom|UnifyReflections
  (for _array_element (Variables|Default|GetReflectionList)
    _))

(event EventBeginPlay
  (bind _outactors (Actor|GetAllActorsOfClass "/Game/BluePrints/ObjectBlueprints/BP_ReflectionEcho.BP_ReflectionEcho_C"))
  (bind _output_get (Variables|Default|SetReflectionList _outactors))
  (Variables|Default|SetTotalPuzzles (Utilities|Array|Length _output_get))
  (for _array_element (Variables|Default|GetReflectionList)
    (CallFunction|PuzzleSolved _array_element)))

(event Collision|EventActorBeginOverlap
  (params (OtherActor :type Actor%20Object%20Reference)))

(event EventTick
  (params (DeltaSeconds :type Float%20%28single-precision%29)))

(fn ConstructionScript)