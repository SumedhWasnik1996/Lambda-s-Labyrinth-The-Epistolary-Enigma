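; BP_FortuneTeller is an interactable fortune teller that sends the player through a repeating loop before moving on to the library level.
; Interaction events toggle a prompt widget, and Interact uses a State counter to step through RecursivePhrases.
; Each step prints a phrase and moves the player back to the first PlayerStart found.
; When the counter reaches the last index, it prints a closing loop line, destroys itself and opens L4_Libarary.
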(event EventBeginPlay)

(event Collision|EventActorBeginOverlap
  (params (OtherActor :type Actor%20Object%20Reference)))

(event EventTick
  (params (DeltaSeconds :type Float%20%28single-precision%29)))

(event EventShowInteractionPrompt
  (params (InteractActor :type Actor%20Object%20Reference))
  (Rendering|SetVisibility (Variables|Default|GetPromptWidget) true false))

(event EventHideInteractionPrompt
  (Rendering|SetVisibility (Variables|Default|GetPromptWidget) false false))

(event EventInteract
  (params (InteractingActor :type Actor%20Object%20Reference))
  (if (< (Variables|Default|GetState) (- (Utilities|Array|Length (Variables|Default|GetRecursivePhrases)) 1))
    (bind _result (Math|Integer|IncrementInt (Variables|Default|GetState))
      (:%20%20
        (Development|PrintString (Utilities|Array|Get(acopy) (Variables|Default|GetRecursivePhrases) _result))
        (Rendering|SetVisibility (Variables|Default|GetPromptWidget) true false)
        (bind _outactors (Actor|GetAllActorsOfClass "/Script/Engine.PlayerStart"))
        (Transformation|SetActorLocation (Game|GetPlayerCharacter 0) (Transformation|GetActorLocation (Utilities|Array|Get(acopy) _outactors)) false false)))
    (else
      (Development|PrintString "The pattern repeats. It is a loop.")
      (Actor|DestroyActor)
      (Game|OpenLevel(byObjectReference) "/Game/Maps/L4_Libarary.L4_Libarary"))))

(fn ConstructionScript)