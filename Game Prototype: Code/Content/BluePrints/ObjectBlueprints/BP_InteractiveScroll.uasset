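; BP_InteractiveScroll is an interactive scroll actor that opens a currying puzzle and leads to the L5_Vault level once solved.
; Interaction prompt events show and hide its PromptWidget.
; Interact creates UMG_CurryingInterface, passes itself as parent actor and switches input to UI only.
; OnPuzzleSolved prints an attunement message, destroys the scroll and opens the vault level.
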(event Custom|OnPuzzleSolved
  (Development|PrintString "You are attuned")
  (Actor|DestroyActor)
  (Game|OpenLevel(byObjectReference) "/Game/Maps/L5_Vault.L5_Vault"))

(event EventBeginPlay)

(event Collision|EventActorBeginOverlap
  (params (OtherActor :type Actor%20Object%20Reference)))

(event EventTick
  (params (DeltaSeconds :type Float%20%28single-precision%29)))

(event EventShowInteractionPrompt
  (params (InteractActor :type Actor%20Object%20Reference))
  (Rendering|SetVisibility (Variables|Default|GetPromptWidget) true false))

(event EventHideInteractionPrompt
  (Rendering|SetVisibility (Variables|Default|GetPromptWidget) false false))

(event EventInteract
  (params (InteractingActor :type Actor%20Object%20Reference))
  (bind _returnvalue (UserInterface|CreateWidget "/Game/UI/UMG_CurryingInterface.UMG_CurryingInterface_C"))
  (Default|SetParentActor _returnvalue self)
  (UserInterface|Viewport|AddtoViewport _returnvalue 0)
  (Input|SetInputModeUIOnly (Game|GetPlayerController 0) _returnvalue "DoNotLock" false))

(fn ConstructionScript)