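; BP_ReflectionEcho is an echo actor that displays an altered dialogue line and opens a dialogue UI when the player approaches.
; On BeginPlay it looks up DialogueID in DialogueTable, writes the altered line to its subtitle widget component and caches the echo puzzle manager.
; When the third-person character enters the trigger box and HasShownWidget is false, it creates WBP_EchoDialogue and switches to UI-only input with a visible cursor.
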(event OnComponentBeginOverlap(Trigger_Box)
  (params (OverlappedComponent :type Primitive%20Component%20Object%20Reference) (OtherActor :type Actor%20Object%20Reference) (OtherComp :type Primitive%20Component%20Object%20Reference) (OtherBodyIndex :type Integer) (bFromSweep :type Boolean) (SweepResult :type Hit%20Result%20Structure%20%28by%20ref%29))
  (bind _returnvalue (Game|GetPlayerController 0))
  (Utilities|Casting|CastToBP_ThirdPersonCharacter OtherActor)
  (if (not (Variables|Default|GetbHasShownWidget))
    (bind _returnvalue_2 (UserInterface|CreateWidget "/Game/UI/WBP_EchoDialogue.WBP_EchoDialogue_C"))
    (bind _output_get (Variables|Default|SetWidgetRef _returnvalue_2))
    (UserInterface|Viewport|AddtoViewport _output_get 0)
    (Input|SetInputModeUIOnly _returnvalue _output_get "DoNotLock" false)
    (Variables|/Script/Engine.PlayerController|SetbShowMouseCursor _returnvalue true)))

(event EventBeginPlay
  (bind _returnvalue (Utilities|GetDataTableRow (Variables|Default|GetDialogueTable) (Variables|Default|GetDialogueID))
    (:then
      (Variables|Default|SetDialogueRow _returnvalue)
      (bind _aswbp_echo_subtitle (Utilities|Casting|CastToWBP_EchoSubtitle (UserInterface|GetUserWidgetObject (Variables|Default|GetWidget_Subtitle))))
      (Default|SetSubtitleText _aswbp_echo_subtitle (.AlteredLine (Utilities|Struct|BreakF_EchoDialogue _returnvalue)))
      (bind _outactors (Actor|GetAllActorsOfClass "/Game/BluePrints/ObjectBlueprints/BP_EchoPuzzleManager.BP_EchoPuzzleManager_C"))
      (Variables|Default|SetPuzzleManagerRef (Utilities|Array|Get(acopy) _outactors)))))

(event Collision|EventActorBeginOverlap
  (params (OtherActor :type Actor%20Object%20Reference)))

(event EventTick
  (params (DeltaSeconds :type Float%20%28single-precision%29)))

(fn ConstructionScript)